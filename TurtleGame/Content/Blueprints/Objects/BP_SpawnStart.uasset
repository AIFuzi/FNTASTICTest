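; BP_SpawnStart is a spawn point actor that creates a turtle and sends it toward an assigned finish.
; On BeginPlay it registers itself as the SpawnStart of its AssignedFinish.
; SpawnTurtle destroys any current turtle, spawns a new one at the SpawnSphere transform, and passes the finish location to the turtle's moving component.
; A getter exposes the current turtle.
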(event EventBeginPlay
  (Utilities|IsValid (Variables|Default|GetAssignedFinish)
    (:Is%20Valid
      (Variables|/Game/Blueprints/Objects/BP_Finish.BP_Finish_C|SetSpawnStart (Variables|Default|GetAssignedFinish) self))))

(fn ConstructionScript)

(fn SpawnTurtle
  (Utilities|IsValid (Variables|Default|GetCurrentSpawnedTurtle)
    (:Is%20Valid
      (Actor|DestroyActor (Variables|Default|GetCurrentSpawnedTurtle)))
    (:Is%20Not%20Valid
      _))
  (bind _returnvalue (Game|SpawnActorfromClass (Variables|Default|GetTurtleClass) (Math|Transform|MakeTransform (Transformation|GetWorldLocation (Variables|Default|GetSpawnSphere)) (Transformation|GetWorldRotation (Variables|Default|GetSpawnSphere)) "1,1,1") "AlwaysSpawn" 0 0))
  (bind _output_get (Variables|Default|SetCurrentSpawnedTurtle _returnvalue))
  (Default|SetFinishPoint (Variables|/Game/Blueprints/Characters/Mario/BP_Mario.BP_Mario_C|GetBP_TurtleMovingComponent _output_get) (Transformation|GetActorLocation (Variables|Default|GetAssignedFinish))))

(fn GetCurrentSpawnedTurtle
  (return (Variables|Default|GetCurrentSpawnedTurtle)))