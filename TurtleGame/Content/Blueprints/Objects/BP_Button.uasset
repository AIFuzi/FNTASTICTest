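; BP_Button is an interactable button that tells its assigned spawner to spawn a turtle.
; The construction script builds its text label from a number and description, and BeginPlay creates a dynamic material and registers the button with the spawner.
; Interact succeeds only when unblocked with a valid spawner, then blocks the button.
; BlockButton sets that state and colors the material red when blocked, green when free.
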(event EventBeginPlay
  (bind _returnvalue (Rendering|Material|CreateDynamicMaterialInstance (Variables|Default|GetCube) 0 "/Game/Assets/Materials/M_Button.M_Button" "None" :!class /Script/Engine.PrimitiveComponent))
  (Variables|Default|SetButtonMaterial _returnvalue)
  (Utilities|IsValid (Variables|Default|GetAssignedSpawner)
    (:Is%20Valid
      (Variables|/Game/Blueprints/Objects/BP_SpawnStart.BP_SpawnStart_C|SetCurrentButton (Variables|Default|GetAssignedSpawner) self))))

(fn ConstructionScript
  (Rendering|Components|TextRender|SetText (Variables|Default|GetTextRender) (Utilities|Text|FormatText "{num}{\\n}{desc}" (Variables|Default|GetNumber) (Utilities|Text|MakeLiteralText " 
") (Variables|Default|GetDesc))))

(fn BlockButton
  (params (SetBlock :type Boolean))
  (Variables|Default|SetIsButtonBlock SetBlock)
  (Rendering|Material|SetVectorParameterValue (Variables|Default|GetButtonMaterial) "Color" (select (Variables|Default|GetIsButtonBlock) "(R=1.000000,G=0.000000,B=0.000000,A=1.000000)" "(R=0.000000,G=1.000000,B=0.000000,A=1.000000)") :!class /Script/Engine.MaterialInstanceDynamic))

(fn Interact
  (if (not (Variables|Default|GetIsButtonBlock))
    (Utilities|IsValid (Variables|Default|GetAssignedSpawner)
      (:Is%20Valid
        (Default|SpawnTurtle (Variables|Default|GetAssignedSpawner))
        (CallFunction|BlockButton true)
        (return true))
      (:Is%20Not%20Valid
        _)))
  (return false))