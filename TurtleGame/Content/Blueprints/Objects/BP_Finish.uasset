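; BP_Finish is the level finish trigger that reacts when BP_Mario enters its box.
; On overlap, MarioFinish casts the other actor to BP_Mario, sets its finish flag and stops its movement.
; If the SpawnStart reference is valid, it calls BlockButton with false on that object's current button, then plays a victory sound and spawns confetti above the finish.
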(event OnComponentBeginOverlap(FinishTriggerBox)
  (params (OverlappedComponent :type Primitive%20Component%20Object%20Reference) (OtherActor :type Actor%20Object%20Reference) (OtherComp :type Primitive%20Component%20Object%20Reference) (OtherBodyIndex :type Integer) (bFromSweep :type Boolean) (SweepResult :type Hit%20Result%20Structure%20%28by%20ref%29))
  (CallFunction|MarioFinish OtherActor))

(fn ConstructionScript)

(fn MarioFinish
  (params (Object :type Actor%20Object%20Reference))
  (bind _returnvalue (Transformation|GetActorLocation))
  (bind _spawnstart (Variables|Default|GetSpawnStart))
  (bind _asbp_mario (Utilities|Casting|CastToBP_Mario Object))
  (Variables|/Game/Blueprints/Characters/Mario/BP_Mario.BP_Mario_C|SetIsFinish _asbp_mario true)
  (Default|StopMoving _asbp_mario)
  (Utilities|IsValid _spawnstart
    (:Is%20Valid
      (Default|BlockButton (Variables|/Game/Blueprints/Objects/BP_SpawnStart.BP_SpawnStart_C|GetCurrentButton _spawnstart) false)
      (Audio|PlaySoundatLocation "/Game/Assets/Sounds/S_Victory.S_Victory" _returnvalue "0, 0, 0" 1.0 1.0 0.0 "/Game/Assets/Sounds/Footstep/FootstepsSoundAttenuation.FootstepsSoundAttenuation" 0 0)
      (Effects|SpawnEmitteratLocation "/Game/Assets/FX/P_Confetti.P_Confetti" (+ _returnvalue "0, 0,200.000000")))))