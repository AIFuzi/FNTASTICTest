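; BP_Mario is a Mario character that walks itself toward or away from a GoalLocation using AI simple move-to navigation.
; On possession it starts a looping timer that re-issues the move order every MovingRate seconds.
; A second timer drives backward movement by rotating the goal offset 180 degrees around the actor's position.
; Stop functions clear each timer and halt CharacterMovement immediately; the backward pair is not called within this Blueprint.
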(event EventPossessed
  (params (NewController :type Controller%20Object%20Reference))
  (CallFunction|StartMoving))

(fn ConstructionScript)

(fn StartMoving
  (bind _returnvalue (Utilities|Time|SetTimerbyFunctionName 0 "CharMoving" (Variables|Default|GetMovingRate) true))
  (Variables|Default|SetMovingTimer _returnvalue))

(fn StopMoving
  (Utilities|Time|ClearandInvalidateTimerbyHandle (Variables|Default|GetMovingTimer))
  (Components|Movement|StopMovementImmediately (Variables|Character|GetCharacterMovement)))

(fn CharMoving
  (AI|Navigation|SimpleMovetoLocation (Pawn|GetController) (Variables|Default|GetGoalLocation)))

(fn MoveBackward
  (AI|Navigation|SimpleMovetoLocation (Pawn|GetController) (+ (Math|Vector|RotateVector (- (Variables|Default|GetGoalLocation) (Transformation|GetActorLocation)) "0,-180.000000, 0") (Transformation|GetActorLocation))))

(fn StartMovingBack
  (bind _returnvalue (Utilities|Time|SetTimerbyFunctionName 0 "MoveBackward" (Variables|Default|GetMovingRate) true))
  (Variables|Default|SetBackMovingTimer _returnvalue))

(fn StopMovingBackward
  (Utilities|Time|ClearandInvalidateTimerbyHandle (Variables|Default|GetBackMovingTimer))
  (Components|Movement|StopMovementImmediately (Variables|Character|GetCharacterMovement)))