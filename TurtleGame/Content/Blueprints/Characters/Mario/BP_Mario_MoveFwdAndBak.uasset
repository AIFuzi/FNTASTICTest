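; Mario character variant that alternates between moving forward and moving backward, overriding movement functions inherited from its parent Blueprint.
; StartMoving and StartMovingBack each halt the opposite motion, call the parent version and schedule the other through a function-name timer.
; The forward phase lasts longer than the backward one, and the loop ends when IsFinish is set as StartMovingBack fires.
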(fn ConstructionScript
  (|CallParentFunction))

(fn StartMoving
  (|CallParentFunction)
  (CallFunction|StopMovingBackward)
  (Utilities|Time|SetTimerbyFunctionName 0 "StartMovingBack" 1.0))

(fn StartMovingBack
  (if (not (Variables|Default|GetIsFinish))
    (CallFunction|StopMoving)
    (|CallParentFunction)
    (Utilities|Time|SetTimerbyFunctionName 0 "StartMoving" 0.5)))