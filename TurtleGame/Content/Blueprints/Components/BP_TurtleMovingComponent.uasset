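; BP_TurtleMovingComponent is an actor component that moves its owning character toward a settable finish point.
; On BeginPlay it caches the owner as CurrentCharacter, which requires a successful cast to BP_Mario despite the turtle name.
; StartMoving runs a looping timer at MovingRate that reissues SimpleMoveToLocation through the character's controller toward FinishPoint.
; StopMoving clears that timer without explicitly cancelling the current move, and SetFinishPoint updates the goal.
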(event EventBeginPlay
  (bind _asbp_mario (Utilities|Casting|CastToBP_Mario (Components|GetOwner)))
  (Variables|Default|SetCurrentCharacter _asbp_mario))

(fn StartMoving
  (bind _returnvalue (Utilities|Time|SetTimerbyFunctionName 0 "CharMoving" (Variables|Default|GetMovingRate) true))
  (Variables|Timers|SetMovingTimer _returnvalue))

(fn CharMoving
  (AI|Navigation|SimpleMovetoLocation (Pawn|GetController (Variables|Default|GetCurrentCharacter)) (Variables|Default|GetFinishPoint)))

(fn StopMoving
  (Utilities|Time|ClearandInvalidateTimerbyHandle (Variables|Timers|GetMovingTimer)))

(fn SetFinishPoint
  (params (Finish :type Vector))
  (Variables|Default|SetFinishPoint Finish))